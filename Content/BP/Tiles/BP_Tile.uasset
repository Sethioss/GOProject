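; BP_Tile is a tile actor whose plane mesh displays its walkable state and its up, down, left and right flags.
; The construction script creates a dynamic instance of M_Line, feeds those booleans in as scalar parameters and applies it to the plane.
; The event graph holds only disabled stub events, so the tile runs no gameplay logic of its own there.
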(fn `UserConstructionScript`
  (bind _returnvalue (`KismetMaterialLibrary.CreateDynamicMaterialInstance` "/Game/Materials/M_Line.M_Line"))
  (`MaterialInstanceDynamic.SetScalarParameterValue` _returnvalue "IsWalkable" (`KismetMathLibrary.Conv_BoolToDouble` (`self.IsWalkableNode`)))
  (`MaterialInstanceDynamic.SetScalarParameterValue` _returnvalue "Top" (`KismetMathLibrary.Conv_BoolToDouble` (`self.Up`)))
  (`MaterialInstanceDynamic.SetScalarParameterValue` _returnvalue "Down" (`KismetMathLibrary.Conv_BoolToDouble` (`self.Down`)))
  (`MaterialInstanceDynamic.SetScalarParameterValue` _returnvalue "Left" (`KismetMathLibrary.Conv_BoolToDouble` (`self.Left`)))
  (`MaterialInstanceDynamic.SetScalarParameterValue` _returnvalue "Right" (`KismetMathLibrary.Conv_BoolToDouble` (`self.Right`)))
  (`PrimitiveComponent.SetMaterial` (`self.PlaneMesh`) 0 _returnvalue))